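; An actor component for Goal actors that shows the goal's team as on-screen HUD text.
; BeginPlay creates a GoalText widget, hands it the owning actor and adds it to the viewport.
; Every Tick it casts the owner to Goal, maps its Team to a player, neutral or enemy label, and pushes that into the widget's text block by polling.
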(event EventBeginPlay
  (bind _returnvalue (UserInterface|CreateWidget "/Game/HUDBlueprints/GoalText.GoalText_C"))
  (Variables|Default|SetGoalTextWidget _returnvalue)
  (Variables|/Game/HUDBlueprints/GoalText.GoalText_C|SetGoalComponent (Variables|Default|GetGoalTextWidget) (Components|GetOwner))
  (Variables|/Game/HUDBlueprints/GoalText.GoalText_C|SetGoalText (Variables|Default|GetGoalTextWidget) "")
  (UserInterface|Viewport|AddtoViewport (Variables|Default|GetGoalTextWidget) 0))

(event EventTick
  (params (DeltaSeconds :type Float%20%28single-precision%29))
  (bind _asgoal (Utilities|Casting|CastToGoal (Components|GetOwner)))
  (switch Utilities|FlowControl|Switch|SwitchonETeam (Variables|/Script/FinalProject.Goal|Getteam _asgoal)
    (:PLAYER
      (Variables|Default|SetGoalText "player"))
    (:NEUTRAL
      (Variables|Default|SetGoalText "neutral"))
    (:ENEMY
      (Variables|Default|SetGoalText "enemy")))
  (Rendering|Components|TextRender|SetText (Variables|/Game/HUDBlueprints/GoalText.GoalText_C|GetGoalTextBlock (Variables|Default|GetGoalTextWidget)) (Variables|Default|GetGoalText)))